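; BP_CheckPoint is a checkpoint actor that sets the player's respawn point.
; When a BP_PlayerPawn overlaps its collider, it compares the pawn's RespawnPoint to the collider's world transform, so the already active checkpoint is ignored.
; Otherwise it stores that transform on the pawn, flags CheckPointReached and plays a whoosh sound at the mesh.
; After a short delay it hides the checkpoint particle.
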(event OnComponentBeginOverlap(CheckPoint_Collider)
  (params (OverlappedComponent :type Primitive%20Component%20Object%20Reference) (OtherActor :type Actor%20Object%20Reference) (OtherComp :type Primitive%20Component%20Object%20Reference) (OtherBodyIndex :type Integer) (bFromSweep :type Boolean) (SweepResult :type Hit%20Result%20Structure%20%28by%20ref%29))
  (bind _asbp_player_pawn (Utilities|Casting|CastToBP_PlayerPawn OtherActor))
  (if (not (== (Variables|/Game/Blueprints/Player/BP_PlayerPawn.BP_PlayerPawn_C|GetRespawnPoint _asbp_player_pawn) (Transformation|GetWorldTransform (Variables|Default|GetCheckPoint_Collider))))
    (Variables|/Game/Blueprints/Player/BP_PlayerPawn.BP_PlayerPawn_C|SetRespawnPoint _asbp_player_pawn (Transformation|GetWorldTransform (Variables|Default|GetCheckPoint_Collider)))
    (Variables|/Game/Blueprints/Player/BP_PlayerPawn.BP_PlayerPawn_C|SetcheckPointReached? _asbp_player_pawn true)
    (Audio|PlaySoundatLocation "/Game/Sound/Effects/whoosh_powerful_energy_pass_Cue.whoosh_powerful_energy_pass_Cue" (Transformation|GetWorldLocation (Variables|Default|GetSM_CheckPoint)) "0, 0, 0" 1.0 1.0 0.0 0 0 0)
    (Utilities|FlowControl|Delay 0.5)
    (Rendering|SetVisibility (Variables|Default|GetCheckPoint_Particle) false false)))

(event EventBeginPlay)

(event Collision|EventActorBeginOverlap
  (params (OtherActor :type Actor%20Object%20Reference)))

(event EventTick
  (params (DeltaSeconds :type Float%20%28single-precision%29)))

(fn ConstructionScript)