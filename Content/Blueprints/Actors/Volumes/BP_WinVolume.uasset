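; BP_WinVolume is a volume actor that completes the level when the player overlaps it with no crystals left.
; On overlap it counts remaining BP_Crystal actors via GetAllActorsOfClass.
; It finds the current level in the LevelNames array and opens the next entry by name.
; On the last entry it instead pauses the game, shows the cursor and displays the WB_EndingScreen widget.
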(event Collision|EventActorBeginOverlap
  (params (OtherActor :type Actor%20Object%20Reference))
  (Utilities|IsPlayer? OtherActor
    (:IsPlayer
      (if (not (.ReturnValue (CallFunction|AnyCrystalsRemaining)))
        (LevelManagement|CompleteLevel)))))

(fn ConstructionScript)

(fn AnyCrystalsRemaining
  (bind _outactors (Actor|GetAllActorsOfClass "/Game/Blueprints/Actors/Collectables/BP_Crystal.BP_Crystal_C"))
  (return (> (Utilities|Array|Length _outactors) 0) (Utilities|Array|Length _outactors)))

(fn CompleteLevel
  (if (LevelManagement|IsFinalLevel)
    (CallFunction|ShowEndingScreen)
    (else
      (LevelManagement|LoadNextLevel))))

(fn GetCurrentLevelIndex
  (bind _returnvalue (Game|GetCurrentLevelName true))
  (return (Utilities|Array|FindItem (Variables|Default|GetLevelNames) (Utilities|String|StringToName _returnvalue))))

(fn IsFinalLevel
  (return (== (Utilities|Array|LastIndex (Variables|Default|GetLevelNames)) (LevelManagement|GetCurrentLevelIndex))))

(fn LoadNextLevel
  (Game|OpenLevel(byName) (LevelManagement|GetNextLevelName)))

(fn GetNextLevelName
  (return (Utilities|Array|Get(acopy) (Variables|Default|GetLevelNames) (+ (LevelManagement|GetCurrentLevelIndex) 1))))

(fn ShowEndingScreen
  (bind _returnvalue (Game|GetPlayerController 0))
  (Game|SetGamePaused true)
  (Input|SetInputModeGameandUI _returnvalue 0 "DoNotLock" true)
  (Variables|/Script/Engine.PlayerController|SetbShowMouseCursor _returnvalue true)
  (bind _returnvalue_2 (UserInterface|CreateWidget "/Game/Blueprints/UI/WB_EndingScreen.WB_EndingScreen_C" _returnvalue))
  (UserInterface|Viewport|AddtoViewport _returnvalue_2 0))