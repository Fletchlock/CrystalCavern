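; BP_Cannon is an automatic cannon that repeatedly fires BP_Projectile actors if ActivateCannon is set at BeginPlay.
; Each cycle waits FireRate, spawns a scaled projectile at ProjectileSpawnPoint, then plays launch sound and smoke.
; The CannonBarrelAnimate timeline moves the barrel along relative Y, and its Cannon Fired event track loops back to the delay, sustaining fire without Tick.
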(event EventBeginPlay
  (if (Variables|CannonFiringSettings|GetActivateCannon)
    (Utilities|FlowControl|Delay (Variables|CannonFiringSettings|GetFireRate) :!label _label)
    (CallFunction|SpawnProjectile)
    (Audio|PlaySoundatLocation "/Game/Sound/Effects/projectile_launch_Cue.projectile_launch_Cue" (Transformation|GetWorldLocation (Variables|Default|GetCannonBarrel)) "0, 0, 0" 0.75 1.0 0.0 0 0 0)
    (Effects|SpawnEmitteratLocation "/Game/Blueprints/Actors/Weapons/PS_Smoke.PS_Smoke" (Transformation|GetWorldLocation (Variables|Default|GetP_Smoke)) "0, 0, 0" "1.000000,1.000000,1.000000" false)
    (bind _cannonbarrelylocation (Timeline|CannonBarrelAnimate PlayFromStart)
      (:Update
        (CallFunction|MoveCannonBarrel _cannonbarrelylocation))
      (:CannonFired
        (goto _label)))))

(event Collision|EventActorBeginOverlap
  (params (OtherActor :type Actor%20Object%20Reference)))

(event EventTick
  (params (DeltaSeconds :type Float%20%28single-precision%29)))

(fn ConstructionScript)

(fn SpawnProjectile
  (bind _projectilespawnpoint (Variables|Default|GetProjectileSpawnPoint))
  (Game|SpawnActorfromClass "/Game/Blueprints/Actors/Projectiles/BP_Projectile.BP_Projectile_C" (Math|Transform|MakeTransform (Transformation|GetWorldLocation _projectilespawnpoint) (Transformation|GetWorldRotation _projectilespawnpoint) (Math|Conversions|ToVector(Float) (Variables|CannonFiringSettings|GetProjectileScale))) "Undefined" 0 0))

(fn MoveCannonBarrel
  (params (CannonBarrelYLocation :type Float%20%28single-precision%29))
  (Transformation|SetRelativeLocation (Variables|Default|GetCannonBarrel) (Math|Vector|MakeVector 0.0 CannonBarrelYLocation 0.0) false false))