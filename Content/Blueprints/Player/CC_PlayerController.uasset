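; Player controller that creates and toggles the player HUD widget.
; BeginPlay creates WB_HUD and stores it in HUDRef without adding it to the viewport.
; ToggleHUD removes HUDRef from its parent when valid, otherwise builds a new HUD with crystals-remaining and level-name child widgets in placeholders.
; That new HUD is never saved to HUDRef, and removal does not clear the reference.
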(event Custom|ToggleHUD
  (bind _hud_ref (Variables|Default|GetHUD_Ref)
    (:then
      (Widget|RemovefromParent _hud_ref))
    (:else
      (bind _returnvalue (UserInterface|CreateWidget "/Game/Blueprints/UI/WB_HUD.WB_HUD_C"))
      (UserInterface|Viewport|AddtoViewport _returnvalue 0)
      (bind _returnvalue_2 (UserInterface|CreateWidget "/Game/Blueprints/UI/WB_CrystalsRemaining.WB_CrystalsRemaining_C"))
      (Widget|Panel|AddChild (Variables|/Game/Blueprints/UI/WB_HUD.WB_HUD_C|GetCrystalRemaining_ph _returnvalue) _returnvalue_2)
      (bind _returnvalue_3 (UserInterface|CreateWidget "/Game/Blueprints/UI/WB_LevelName.WB_LevelName_C"))
      (Widget|Panel|AddChild (Variables|/Game/Blueprints/UI/WB_HUD.WB_HUD_C|GetLevelName_ph _returnvalue) _returnvalue_3))))

(event EventBeginPlay
  (bind _returnvalue (UserInterface|CreateWidget "/Game/Blueprints/UI/WB_HUD.WB_HUD_C"))
  (Variables|Default|SetHUD_Ref _returnvalue))

(event EventTick
  (params (DeltaSeconds :type Float%20%28single-precision%29)))

(fn ConstructionScript)