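; Player pawn for a rolling ball that moves by torque applied to its physics mesh from the movement axes.
; Damage triggers a respawn if a checkpoint was reached, otherwise a glow and a faded level reload.
; Respawning plays the glow on a dynamic material, briefly disables physics and input, then moves the ball to the respawn point.
; It also handles the opening fade, pause menu, HUD toggle and spring-arm adjustment.
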(event Custom|Respawn_Player
  (bind _mesh (Variables|Default|GetMesh))
  (bind _respawnpoint (Variables|Default|GetRespawnPoint))
  (bind _returnvalue (Rendering|Material|CreateDynamicMaterialInstance (Variables|Default|GetMesh) 0 "/Game/Materials/M_BallDamage_Inst.M_BallDamage_Inst" "None" :!class /Script/Engine.PrimitiveComponent))
  (bind _newtrack_0 (Timeline|Timeline_0 Play)
    (:Update
      (Rendering|Material|SetScalarParameterValue _returnvalue "GlowEffect" _newtrack_0 :!class /Script/Engine.MaterialInstanceDynamic)
      (Utilities|FlowControl|Delay 0.6)
      (Input|DisableInput 0)
      (Physics|SetSimulatePhysics (Variables|Default|GetMesh) false)
      (Utilities|FlowControl|Delay 0.1)
      (Physics|SetSimulatePhysics (Variables|Default|GetMesh) true)
      (Input|EnableInput 0)
      (Transformation|SetWorldTransform _mesh (Math|Transform|MakeTransform (Math|Vector|MakeVector (.x (.location _respawnpoint)) (.y (.location _respawnpoint)) (+ (.z (.location _respawnpoint)) 1e+01)) "0, 0, 0" "1.400000,1.400000,1.400000") false false)
      (Rendering|Material|CreateDynamicMaterialInstance _mesh 0 "/Game/StarterContent/Materials/M_Tech_Panel.M_Tech_Panel" "None" :!class /Script/Engine.PrimitiveComponent))))

(event Custom|ToggleHUD
  (bind _hud_ref (Variables|Default|GetHUD_Ref)
    (:then
      (Widget|RemovefromParent _hud_ref))
    (:else
      (bind _returnvalue (UserInterface|CreateWidget "/Game/Blueprints/UI/WB_HUD.WB_HUD_C"))
      (bind _output_get (Variables|Default|SetHUD_Ref _returnvalue))
      (UserInterface|Viewport|AddtoViewport _output_get 0)
      (bind _returnvalue_2 (UserInterface|CreateWidget "/Game/Blueprints/UI/WB_CrystalsRemaining.WB_CrystalsRemaining_C"))
      (Widget|Panel|AddChild (Variables|/Game/Blueprints/UI/WB_HUD.WB_HUD_C|GetCrystalRemaining_ph (Variables|Default|GetHUD_Ref)) _returnvalue_2))))

(event EventBeginPlay
  (CameraFades|StartCameraFade (Game|GetPlayerCameraManager 0) 1.0 0.0 2.0 "(R=0.000000,G=0.000000,B=0.000000,A=1.000000)" true false)
  (bind _returnvalue (UserInterface|CreateWidget "/Game/Blueprints/UI/WB_HUD.WB_HUD_C"))
  (Variables|Default|SetHUD_Ref _returnvalue))

(event Game|Damage|EventAnyDamage
  (params (Damage :type Float%20%28single-precision%29) (DamageType :type Damage%20Type%20Object%20Reference) (InstigatedBy :type Controller%20Object%20Reference) (DamageCauser :type Actor%20Object%20Reference))
  (if (Variables|Default|GetcheckPointReached?)
    (CallFunction|RespawnPlayer)
    (else
      (bind _returnvalue (Rendering|Material|CreateDynamicMaterialInstance (Variables|Default|GetMesh) 0 "/Game/Materials/M_BallDamage_Inst.M_BallDamage_Inst" "None" :!class /Script/Engine.PrimitiveComponent))
      (bind _newtrack_0 (Timeline|GlowTransition Play)
        (:Update
          (Rendering|Material|SetScalarParameterValue _returnvalue "GlowEffect" _newtrack_0 :!class /Script/Engine.MaterialInstanceDynamic)
          (Utilities|RestartLevel))))))

(event Input|AxisEvents|InputAxisMoveForwards/Backwards
  (params (AxisValue :type Float%20%28single-precision%29))
  (Class|PrimitiveComponent|AddTorqueinRadians (Variables|Default|GetMesh) (Math|Vector|MakeVector 0.0 (* AxisValue (Variables|BallSetings|GetAccelerationMultiplier)) 0.0) "None" true))

(event Input|AxisEvents|InputAxisMoveRight/Left
  (params (AxisValue :type Float%20%28single-precision%29))
  (Class|PrimitiveComponent|AddTorqueinRadians (Variables|Default|GetMesh) (Math|Vector|MakeVector (* AxisValue (Variables|BallSetings|GetAccelerationMultiplier)) 0.0 0.0) "None" true))

(event Input|KeyboardEvents|Escape
  (params (Key :type Key%20Structure :default "None"))
  (bind _returnvalue (Game|GetPlayerController 0))
  (:Pressed
    (Game|SetGamePaused true)
    (Input|SetInputModeGameandUI _returnvalue 0 "DoNotLock" true)
    (Variables|/Script/Engine.PlayerController|SetbShowMouseCursor _returnvalue true)
    (bind _returnvalue_2 (UserInterface|CreateWidget "/Game/Blueprints/UI/WB_PauseMenu.WB_PauseMenu_C" _returnvalue))
    (UserInterface|Viewport|AddtoViewport _returnvalue_2 0)))

(event Input|KeyboardEvents|P
  (params (Key :type Key%20Structure :default "None"))
  (bind _returnvalue (Game|GetPlayerController 0))
  (:Pressed
    (Game|SetGamePaused true)
    (Input|SetInputModeGameandUI _returnvalue 0 "DoNotLock" true)
    (Variables|/Script/Engine.PlayerController|SetbShowMouseCursor _returnvalue true)
    (bind _returnvalue_2 (UserInterface|CreateWidget "/Game/Blueprints/UI/WB_PauseMenu.WB_PauseMenu_C" _returnvalue))
    (UserInterface|Viewport|AddtoViewport _returnvalue_2 0)))

(fn ConstructionScript)

(fn AdjustSpringArm
  (params (Distance :type Float%20%28single-precision%29) (Pitch :type Float%20%28single-precision%29) (Rotation :type Float%20%28single-precision%29))
  (bind _springarm (Variables|Default|GetSpringArm))
  (Variables|/Script/Engine.SpringArmComponent|SetTargetArmLength _springarm Distance)
  (Transformation|SetWorldRotation _springarm (Math|Rotator|MakeRotator 0.0 Pitch Rotation) false false))